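; AI shooter character Blueprint that colors its mannequin by team and visualizes where it is looking.
; On BeginPlay it sets both mesh material slots to Red, Green or Blue Manny material instances selected by the CharacterTeam value.
; Every tick it draws a debug arrow from the actor's eyes view point along the view rotation.
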(event `self.ReceiveBeginPlay`
  (bind _characterteam (`self.CharacterTeam`))
  (bind _mesh (`self.Mesh`))
  (`PrimitiveComponent.SetMaterial` _mesh 0 (select `ETeams` _characterteam :`Red` "/Game/AI_Shooter/3D_Assets/Characters/Mannequins/Materials/Instances/Manny/MI_Manny_02_Red.MI_Manny_02_Red" :`Green` "/Game/AI_Shooter/3D_Assets/Characters/Mannequins/Materials/Instances/Manny/MI_Manny_02_Green.MI_Manny_02_Green" :`Blue` "/Game/AI_Shooter/3D_Assets/Characters/Mannequins/Materials/Instances/Manny/MI_Manny_02_Blue.MI_Manny_02_Blue" :!type "MaterialInterface Object Reference"))
  (`PrimitiveComponent.SetMaterial` _mesh 1 (select `ETeams` _characterteam :`Red` "/Game/AI_Shooter/3D_Assets/Characters/Mannequins/Materials/Instances/Manny/MI_Manny_01_Red.MI_Manny_01_Red" :`Green` "/Game/AI_Shooter/3D_Assets/Characters/Mannequins/Materials/Instances/Manny/MI_Manny_01_Green.MI_Manny_01_Green" :`Blue` "/Game/AI_Shooter/3D_Assets/Characters/Mannequins/Materials/Instances/Manny/MI_Manny_01_Blue.MI_Manny_01_Blue" :!type "MaterialInterface Object Reference")))

(event `self.ReceiveTick`
  (params (DeltaSeconds :type "Float (single-precision)"))
  (bind (_outlocation _outrotation) (`self.GetActorEyesViewPoint`))
  (`KismetSystemLibrary.DrawDebugArrow` _outlocation (+ _outlocation (* (`KismetMathLibrary.Conv_RotatorToVector` _outrotation) 100.0)) 0.0 (struct :`A` 1.0) 0.0 10.0))

(fn `UserConstructionScript`)